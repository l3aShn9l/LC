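; BP_CampaignHexTile is a campaign map hex tile whose colour reflects its landscape type.
; The construction script creates a dynamic material instance on the static mesh.
; UpdateColour switches on the Landscape enum (mountains, plains, woods, lake, town) to set that material's Base Color parameter.
; It runs on BeginPlay and from the Landscape OnRep, so replicated landscape changes recolour the tile.
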(event EventBeginPlay
  (CallFunction|UpdateColour))

(fn ConstructionScript
  (bind _returnvalue (Rendering|Material|CreateDynamicMaterialInstance (Variables|Default|GetStaticMesh) 0 "/Game/LC/Game/CampaignHexTileMaterialMaterial.CampaignHexTileMaterialMaterial" "None" :!class /Script/Engine.PrimitiveComponent))
  (Variables|Default|SetDMI _returnvalue))

(fn OnRepLandscape
  (CallFunction|UpdateColour))

(fn UpdateColour
  (switch Utilities|FlowControl|Switch|SwitchonE_Landscape (Variables|Default|GetLandscape)
    (:NewEnumerator2
      (Rendering|Material|SetVectorParameterValue (Variables|Default|GetDMI) "Base Color" (Utilities|Struct|MakeLinearColor 0.25 0.25 0.25 1.0) :!class /Script/Engine.MaterialInstanceDynamic))
    (:NewEnumerator0
      (Rendering|Material|SetVectorParameterValue (Variables|Default|GetDMI) "Base Color" (Utilities|Struct|MakeLinearColor 0.25 1.0 0.25 1.0) :!class /Script/Engine.MaterialInstanceDynamic))
    (:NewEnumerator1
      (Rendering|Material|SetVectorParameterValue (Variables|Default|GetDMI) "Base Color" (Utilities|Struct|MakeLinearColor 0.003922 0.196078 0.117647 1.0) :!class /Script/Engine.MaterialInstanceDynamic))
    (:NewEnumerator3
      (Rendering|Material|SetVectorParameterValue (Variables|Default|GetDMI) "Base Color" (Utilities|Struct|MakeLinearColor 0.0 0.0 1.0 1.0) :!class /Script/Engine.MaterialInstanceDynamic))
    (:NewEnumerator4
      (Rendering|Material|SetVectorParameterValue (Variables|Default|GetDMI) "Base Color" (Utilities|Struct|MakeLinearColor 0.012658 0.025641 0.0 1.0) :!class /Script/Engine.MaterialInstanceDynamic))))