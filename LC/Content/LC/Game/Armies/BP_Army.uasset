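; BP_Army represents an army whose replicated Piece, Faction and Leader drive its visual representation in the game.
; When Faction replicates, it tints the Piece's dynamic material with the faction colour.
; When Leader replicates, it has the ArmyWidget on the Piece's widget component update its image.
; Both updates require a valid Piece, and the Piece's own OnRep is empty, so it does not reapply them.
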(fn OnRepPiece)

(fn OnRepFaction
  (bind _piece (Variables|Default|GetPiece))
  (Utilities|IsValid _piece
    (:Is%20Valid
      (Rendering|Material|SetVectorParameterValue (Variables|/Game/LC/Game/Armies/BP_ArmyPiece.BP_ArmyPiece_C|GetDMI _piece) "Base Color" (Variables|/Game/LC/Game/Factions/BP_Faction.BP_Faction_C|GetColour (Variables|Default|GetFaction)) :!class /Script/Engine.MaterialInstanceDynamic))))

(fn OnRepLeader
  (bind _piece (Variables|Default|GetPiece))
  (Utilities|IsValid _piece
    (:Is%20Valid
      (bind _asarmy_widget (Utilities|Casting|CastToArmyWidget (UserInterface|GetWidget (Variables|/Game/LC/Game/Armies/BP_ArmyPiece.BP_ArmyPiece_C|GetWidget _piece))))
      (Default|SetImage _asarmy_widget))))