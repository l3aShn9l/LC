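; BP_ArmyPiece is the visual piece that represents an Army in the game, with a mesh tinted by faction and an attached widget.
; The construction script creates a dynamic material instance on the army mesh.
; On BeginPlay it passes itself to the ArmyWidget in its widget component, then sets the material's base colour from the army's faction, skipping both steps if the widget cast fails.
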(event EventBeginPlay
  (bind _asarmy_widget (Utilities|Casting|CastToArmyWidget (UserInterface|GetWidget (Variables|Default|GetWidget))))
  (Variables|/Game/LC/Game/Armies/ArmyWidget.ArmyWidget_C|SetArmyPiece _asarmy_widget self)
  (Rendering|Material|SetVectorParameterValue (Variables|Default|GetDMI) "Base Color" (Variables|/Game/LC/Game/Factions/BP_Faction.BP_Faction_C|GetColour (Variables|/Game/LC/Game/Armies/BP_Army.BP_Army_C|GetFaction (Variables|Default|GetArmy))) :!class /Script/Engine.MaterialInstanceDynamic))

(fn ConstructionScript
  (bind _returnvalue (Rendering|Material|CreateDynamicMaterialInstance (Variables|Default|GetArmyMesh) 0 "/Game/LC/Game/Armies/ArmyMaterial.ArmyMaterial" "None" :!class /Script/Engine.PrimitiveComponent))
  (Variables|Default|SetDMI _returnvalue))