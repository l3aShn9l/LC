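; BP_gPC is the player controller that handles mouse selection on the campaign hex map.
; Left click traces under the cursor and stores a clicked army piece's Army as Selected, clearing it otherwise; the per-landscape tile switch currently just clears it.
; Right click ignores the cursor and calls SetColour on the border widget of the game state's hex at (0,0), apparently as a test.
; GetFaction returns the faction from the player state.
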(event EventBeginPlay)

(event Input|MouseEvents|LeftMouseButton
  (params (Key :type Key%20Structure :default "None"))
  (bind _hitresult (Game|Player|GetHitResultUnderCursorbyChannel "TraceTypeQuery2" true))
  (bind _hitactor (Collision|BreakHitResult _hitresult))
  (:Pressed
    (if (== "/Game/LC/Game/Armies/BP_ArmyPiece.BP_ArmyPiece_C" (Utilities|GetClass _hitactor))
      (bind _asbp_army_piece (Utilities|Casting|CastToBP_ArmyPiece _hitactor))
      (Variables|Default|SetSelected (Variables|/Game/LC/Game/Armies/BP_ArmyPiece.BP_ArmyPiece_C|GetArmy _asbp_army_piece))
      (elif (== "/Game/LC/Game/BP_CampaignHexTile.BP_CampaignHexTile_C" (Utilities|GetClass _hitactor))
        (bind _asbp_campaign_hex_tile (Utilities|Casting|CastToBP_CampaignHexTile _hitactor))
        (switch Utilities|FlowControl|Switch|SwitchonE_Landscape (Variables|/Game/LC/Game/BP_CampaignHexTile.BP_CampaignHexTile_C|GetLandscape _asbp_campaign_hex_tile)
          (:NewEnumerator2
            _)
          (:NewEnumerator0
            _)
          (:NewEnumerator1
            _)
          (:NewEnumerator3
            _))
        (Variables|Default|SetSelected 0)
        (else
          (Variables|Default|SetSelected 0))))))

(event Input|MouseEvents|RightMouseButton
  (params (Key :type Key%20Structure :default "None"))
  (:Pressed
    (bind _asbp_g_gs (Utilities|Casting|CastToBP_gGS (Game|GetGameState)))
    (bind _hex (Default|GetHexTile _asbp_g_gs))
    (bind _aswbp_hexagon_border (Utilities|Casting|CastToWBP_HexagonBorder (UserInterface|GetWidget (Variables|/Game/LC/Game/BP_CampaignHexTile.BP_CampaignHexTile_C|GetWidget _hex))))
    (Default|SetColour _aswbp_hexagon_border)))

(fn ConstructionScript)

(fn GetFaction
  (bind _asbp_g_ps (Utilities|Casting|CastToBP_gPS (Variables|GetPlayerState)))
  (return (Variables|/Game/LC/Game/Main/BP_gPS.BP_gPS_C|GetFaction _asbp_g_ps)))