(event EventBeginPlay)

(fn ConstructionScript)

(fn GenerateCampaignMap
  (params (Size%20X :type Integer) (Size%20Y :type Integer))
  (bind _hexes (Variables|Default|GetHexes))
  (Utilities|Array|Clear _hexes)
  (for _index (range 0 (- Size%20Y 1))
    (for _index_2 (range 0 (- Size%20X 1))
      (bind _newparam (CallFunction|IndexestoCoords _index_2 _index))
      (bind _position (CallFunction|CoordstoPosition _newparam))
      (bind _returnvalue (Game|SpawnActorfromClass "/Game/LC/Game/BP_CampaignHexTile.BP_CampaignHexTile_C" (Math|Transform|MakeTransform _position) "Undefined" "MultiplyWithRoot" 0 _newparam "NewEnumerator0" 0))
      (Utilities|Array|Add (LocalVariables|GetTempHexArray) _returnvalue))
    (Utilities|Array|Add _hexes (Utilities|Struct|MakeS_HexArray (LocalVariables|GetTempHexArray)))
    (Utilities|Array|Clear (LocalVariables|GetTempHexArray)))
  (bind (_hex _found) (CallFunction|GetHexTile 0 3))
  (if _found
    (Variables|/Game/LC/Game/BP_CampaignHexTile.BP_CampaignHexTile_C|SetLandscape _hex "NewEnumerator2")
    (bind (_hex_2 _found_2) (CallFunction|GetHexTile 4))
    (if _found_2
      (Variables|/Game/LC/Game/BP_CampaignHexTile.BP_CampaignHexTile_C|SetLandscape _hex_2 "NewEnumerator3"))))

(fn CreateTown
  (bind _returnvalue (Game|ConstructObjectfromClass "/Game/LC/Game/BP_Town.BP_Town_C"))
  (Utilities|Array|Add (Variables|Default|GetTowns) _returnvalue)
  (Class|ORManagerComponent|RegisterReplicatedObject (Variables|Default|GetORManager) _returnvalue)
  (return _returnvalue))

(fn CreateFaction
  (params (Name :type Name) (Colour :type Linear%20Color%20Structure))
  (bind _returnvalue (Game|ConstructObjectfromClass self "/Game/LC/Game/Factions/BP_Faction.BP_Faction_C" Name Colour))
  (Utilities|Array|Add (Variables|Default|GetFactions) _returnvalue)
  (Class|ORManagerComponent|RegisterReplicatedObject (Variables|Default|GetORManager) _returnvalue)
  (return _returnvalue))

(fn CreateLeader
  (params (Name :type Name) (Texture :type Texture%20Object%20Reference) (UnitType :type BP%20Unit%20Class%20Reference))
  (bind _returnvalue (Game|ConstructObjectfromClass "/Game/LC/Game/Leaders/BP_Leader.BP_Leader_C" Name Texture UnitType))
  (Utilities|Array|Add (Variables|Default|GetLeaders) _returnvalue)
  (Class|ORManagerComponent|RegisterReplicatedObject (Variables|Default|GetORManager) _returnvalue)
  (bind _unit (CallFunction|CreateUnit (Variables|/Game/LC/Game/Leaders/BP_Leader.BP_Leader_C|GetUnitType _returnvalue)))
  (Variables|/Game/LC/Game/Leaders/BP_Leader.BP_Leader_C|SetUnit _returnvalue _unit)
  (return _returnvalue))

(fn CreateArmy
  (params (Faction :type BP%20Faction%20Object%20Reference) (Leader :type BP%20Leader%20Object%20Reference) (Coords :type S%20Coordinates%20Structure))
  (bind _returnvalue (Game|ConstructObjectfromClass "/Game/LC/Game/Armies/BP_Army.BP_Army_C" Faction Leader 4 Coords))
  (Utilities|Array|Add (Variables|Default|GetArmies) _returnvalue)
  (Class|ORManagerComponent|RegisterReplicatedObject (Variables|Default|GetORManager) _returnvalue)
  (return _returnvalue))

(fn SpawnArmyPiece
  (params (Army :type BP%20Army%20Object%20Reference))
  (bind _position (CallFunction|CoordstoPosition (Variables|/Game/LC/Game/Armies/BP_Army.BP_Army_C|GetCoords Army)))
  (bind _returnvalue (Game|SpawnActorfromClass "/Game/LC/Game/Armies/BP_ArmyPiece.BP_ArmyPiece_C" (Math|Transform|MakeTransform _position) "Undefined" "MultiplyWithRoot" 0 Army 0))
  (Utilities|Array|Add (Variables|Default|GetArmyPieces) _returnvalue)
  (return _returnvalue))

(fn CreateUnit
  (params (UnitClass :type BP%20Unit%20Class%20Reference))
  (bind _returnvalue (Game|ConstructObjectfromClass UnitClass))
  (return _returnvalue))

(fn SpawnUnitPiece)

(fn GetHexTile
  (params (X :type Integer) (Y :type Integer))
  (bind _hexes (Variables|Default|GetHexes))
  (bind _output (Utilities|Array|Get(acopy) _hexes X))
  (bind _hexarray (Utilities|Struct|BreakS_HexArray _output))
  (bind _output_2 (Utilities|Array|Get(acopy) _hexarray Y))
  (return _output_2 (Utilities|IsValid _output_2)))

(fn GetAvailableHexes
  (params (Army :type BP%20Army%20Piece%20Object%20Reference)))

(fn GetNeighbourHexes
  (params (Hex :type BP%20Campaign%20Hex%20Tile%20Object%20Reference))
  (bind _coords (Variables|/Game/LC/Game/BP_CampaignHexTile.BP_CampaignHexTile_C|GetCoords Hex))
  (bind (_x _y _z) (Utilities|Struct|BreakS_Coordinates _coords))
  (for _array_element (LocalVariables|GetNeighboursOffset)
    (bind (_x_2 _y_2) (CallFunction|CoordstoIndexes (Utilities|Struct|MakeS_Coordinates (+ _x (.X (Utilities|Struct|BreakS_Coordinates _array_element))) (+ _y (.Y (Utilities|Struct|BreakS_Coordinates _array_element))) (+ _z (.Z (Utilities|Struct|BreakS_Coordinates _array_element))))))
    (bind (_hex _found) (CallFunction|GetHexTile _x_2 _y_2))
    (if _found
      (Utilities|Array|Add (LocalVariables|GetTempNeighbours) _hex)))
  (return (LocalVariables|GetTempNeighbours)))