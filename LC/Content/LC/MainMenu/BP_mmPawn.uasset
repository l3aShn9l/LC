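; BP_mmPawn is the main menu pawn that sets up menu input and UI for its player controller.
; On BeginPlay it adds the IMC_MainMenuInput mapping context to the Enhanced Input local player subsystem, then calls AddHUD.
; AddHUD creates the WBP_MainMenu widget for that controller, stores it as HUD and adds it to the viewport.
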(event Custom|AddHUD
  (bind _asplayer_controller (Utilities|Casting|CastToPlayerController (Pawn|GetController)))
  (bind _returnvalue (UserInterface|CreateWidget "/Game/LC/MainMenu/WBP_MainMenu.WBP_MainMenu_C" _asplayer_controller))
  (bind _output_get (Variables|Default|SetHUD _returnvalue))
  (UserInterface|Viewport|AddtoViewport _output_get 0))

(event EventBeginPlay
  (bind _asplayer_controller (Utilities|Casting|CastToPlayerController (Pawn|GetController)))
  (Utilities|IsValid (PlayerController|LocalPlayerSubsystems|GetEnhancedInputLocalPlayerSubsystem _asplayer_controller)
    (:Is%20Valid
      (Input|AddMappingContext (PlayerController|LocalPlayerSubsystems|GetEnhancedInputLocalPlayerSubsystem _asplayer_controller) "/Game/LC/MainMenu/Input/IMC_MainMenuInput.IMC_MainMenuInput" 0 "(bIgnoreAllPressedKeysUntilRelease=True,bForceImmediately=False,bNotifyUserSettings=False)")
      (CallFunction|AddHUD))))

(event Collision|EventActorBeginOverlap
  (params (OtherActor :type Actor%20Object%20Reference)))

(event EventTick
  (params (DeltaSeconds :type Float%20%28single-precision%29)))

(fn ConstructionScript)